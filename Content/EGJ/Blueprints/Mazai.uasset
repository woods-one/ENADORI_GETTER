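; Mazai is an actor, apparently a pickup, that jumps to a random spot in the level when the player touches it.
; BeginPlay places it at random X/Y within fixed bounds at a constant height.
; A capsule overlap matching the player by display-name string relocates it within narrower bounds, with GetMazai blocking retriggers for a one-second delay.
; Any other overlap, including the player's during that delay, only prints the actor's name.
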(event OnComponentBeginOverlap(Capsule)
  (params (OverlappedComponent :type Primitive%20Component%20Object%20Reference) (OtherActor :type Actor%20Object%20Reference) (OtherComp :type Primitive%20Component%20Object%20Reference) (OtherBodyIndex :type Integer) (bFromSweep :type Boolean) (SweepResult :type Hit%20Result%20Structure%20%28by%20ref%29))
  (bind _returnvalue (Utilities|GetDisplayName OtherActor))
  (if (and (Variables|Default|GetGetMazai) (Utilities|Enum|Equal(Enum) "BP_Player_C_0" _returnvalue))
    (Transformation|SetActorLocation (Math|Vector|MakeVector (Math|Conversions|ToFloat(Integer) (Math|Random|RandomIntegerinRange 355 2750)) (Math|Conversions|ToFloat(Integer) (Math|Random|RandomIntegerinRange 360 3150)) 5e+02) false false)
    (Variables|Default|SetGetMazai false)
    (Utilities|FlowControl|Delay 1.0)
    (Variables|Default|SetGetMazai true)
    (else
      (Development|PrintString _returnvalue))))

(event EventBeginPlay
  (Transformation|SetActorLocation (Math|Vector|MakeVector (Math|Conversions|ToFloat(Integer) (Math|Random|RandomIntegerinRange 155 2950)) (Math|Conversions|ToFloat(Integer) (Math|Random|RandomIntegerinRange 160 3350)) 5e+02) false false)
  (Variables|Default|SetGetMazai true))

(fn ConstructionScript)